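; StrategyPawn is a camera pawn with zoom, planar movement and stepped yaw rotation, in the style of a strategy game view.
; Input events only update desired zoom, location and rotation, with zoom clamped and movement relative to the pawn's forward and right vectors.
; Tick smoothly interpolates the spring arm length and actor transform toward those targets, which are seeded from current values at BeginPlay.
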(event EventTick
  (params (DeltaSeconds :type Float%20%28single-precision%29))
  (bind _springarm (Variables|Default|GetSpringArm))
  (Utilities|FlowControl|Sequence
    (:then_0
      (Variables|/Script/Engine.SpringArmComponent|SetTargetArmLength _springarm (Math|Interpolation|FInterpTo (Variables|/Script/Engine.SpringArmComponent|GetTargetArmLength _springarm) (Variables|Default|GetZoom_Desired) DeltaSeconds (Variables|Default|GetZoom_interp_speed))))
    (:then_1
      (Transformation|SetActorLocation (Math|Interpolation|VInterpTo (Transformation|GetActorLocation) (Variables|Default|GetLocation_Desired) DeltaSeconds (Variables|Default|GetLocation_Interp_Speed)) false false))
    (:then_2
      (Transformation|SetActorRotation (Math|Interpolation|RInterpTo (Transformation|GetActorRotation) (Variables|Default|GetRotation_Desired) DeltaSeconds (Variables|Default|GetRotation_Interp_Speed))))))

(event EventBeginPlay
  (Variables|Default|SetZoom_Desired (Variables|/Script/Engine.SpringArmComponent|GetTargetArmLength (Variables|Default|GetSpringArm)))
  (Variables|Default|SetLocation_Desired (Transformation|GetActorLocation))
  (Variables|Default|SetRotation_Desired (Transformation|GetActorRotation)))

(event Input|ActionEvents|InputActionInputAction_RotationLeft
  (params (Key :type Key%20Structure :default "None"))
  (:Pressed
    (Variables|Default|SetRotation_Desired (Math|Rotator|CombineRotators (Variables|Default|GetRotation_Desired) (Math|Rotator|MakeRotator 0.0 0.0 (Variables|Default|GetRotation_speed))))))

(event Input|ActionEvents|InputActionInputAction_RotationRight
  (params (Key :type Key%20Structure :default "None"))
  (:Pressed
    (Variables|Default|SetRotation_Desired (Math|Rotator|CombineRotators (Variables|Default|GetRotation_Desired) (Math|Rotator|MakeRotator 0.0 0.0 (* (Variables|Default|GetRotation_speed) -1.0))))))

(event Input|AxisEvents|InputAxisInputAxis_Zoom
  (params (AxisValue :type Float%20%28single-precision%29))
  (Variables|Default|SetZoom_Desired (Math|Float|Clamp(Float) (+ (* AxisValue (Variables|Default|GetZoom_speed)) (Variables|Default|GetZoom_Desired)) (Variables|Default|GetZoom_Min) (Variables|Default|GetZoom_Max))))

(event Input|AxisEvents|InputAxisInputAxis_Forward
  (params (AxisValue :type Float%20%28single-precision%29))
  (Variables|Default|SetLocation_Desired (+ (Variables|Default|GetLocation_Desired) (* (* AxisValue (Variables|Default|GetLocation_speed)) (Transformation|GetActorForwardVector)))))

(event Input|AxisEvents|InputAxisInputAxis_Right
  (params (AxisValue :type Float%20%28single-precision%29))
  (Variables|Default|SetLocation_Desired (+ (Variables|Default|GetLocation_Desired) (* (* AxisValue (Variables|Default|GetLocation_speed)) (Transformation|GetActorRightVector)))))

(fn ConstructionScript)
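; BP_PlayerActions is an actor that turns player mouse input into actions on the BP_Grid tiles.
; Every tick and click it queries the grid for the tile under the cursor and moves a hover tile state onto it.
; Left and right clicks execute separately selected action actors on that tile.
; SetSelectedAction destroys and respawns those actors from given classes, passing itself in, then broadcasts the change through a dispatcher.
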(event EventBeginPlay
  (bind _returnvalue (Actor|GetActorOfClass "/Game/Blueprints/Core/Grid/BP_Grid.BP_Grid_C"))
  (Variables|Default|SetGrid _returnvalue)
  (Input|EnableInput (Game|GetPlayerController 0)))

(event EventTick
  (params (DeltaSeconds :type Float%20%28single-precision%29))
  (CallFunction|UpdateTileUnderCursor))

(event Input|MouseEvents|LeftMouseButton
  (params (Key :type Key%20Structure :default "None"))
  (:Pressed
    (CallFunction|UpdateTileUnderCursor)
    (Utilities|IsValid (Variables|Default|GetSelectedAction_LeftClick)
      (:Is%20Valid
        (Default|ExecuteAction (Variables|Default|GetSelectedAction_LeftClick) (Variables|Default|GetHoveredTile))))))

(event Input|MouseEvents|RightMouseButton
  (params (Key :type Key%20Structure :default "None"))
  (:Pressed
    (CallFunction|UpdateTileUnderCursor)
    (Utilities|IsValid (Variables|Default|GetSelectedAction_RightClick)
      (:Is%20Valid
        (Default|ExecuteAction (Variables|Default|GetSelectedAction_RightClick) (Variables|Default|GetHoveredTile))))))

(fn ConstructionScript)

(fn UpdateTileUnderCursor
  (bind _index (Default|GetTileIndexUnderCursor (Variables|Default|GetGrid)))
  (if (!= _index (Variables|Default|GetHoveredTile))
    (Default|RemoveStatefromTile (Variables|Default|GetGrid) (Variables|Default|GetHoveredTile) "NewEnumerator1")
    (bind _output_get (Variables|Default|SetHoveredTile _index))
    (Default|AddStatetoTile (Variables|Default|GetGrid) _output_get "NewEnumerator1")))

(fn SetSelectedAction
  (params (LeftAction :type BP%20Action%20Class%20Reference) (RightAction :type BP%20Action%20Class%20Reference))
  (Utilities|FlowControl|Sequence
    (:then_0
      (Utilities|IsValid (Variables|Default|GetSelectedAction_LeftClick)
        (:Is%20Valid
          (Actor|DestroyActor (Variables|Default|GetSelectedAction_LeftClick))
          (Variables|Default|SetSelectedAction_LeftClick 0))
        (:Is%20Not%20Valid
          _))
      (if (Utilities|IsValidClass LeftAction)
        (bind _returnvalue (Game|SpawnActorfromClass LeftAction (Math|Transform|MakeTransform "0, 0, 0" "0, 0, 0" "1.000000,1.000000,1.000000") "AlwaysSpawn" "MultiplyWithRoot" 0 self 0))
        (Variables|Default|SetSelectedAction_LeftClick _returnvalue)))
    (:then_1
      (Utilities|IsValid (Variables|Default|GetSelectedAction_RightClick)
        (:Is%20Valid
          (Actor|DestroyActor (Variables|Default|GetSelectedAction_RightClick))
          (Variables|Default|SetSelectedAction_RightClick 0))
        (:Is%20Not%20Valid
          _))
      (if (Utilities|IsValidClass RightAction)
        (bind _returnvalue_2 (Game|SpawnActorfromClass RightAction (Math|Transform|MakeTransform "0, 0, 0" "0, 0, 0" "1.000000,1.000000,1.000000") "AlwaysSpawn" "MultiplyWithRoot" 0 self 0))
        (Variables|Default|SetSelectedAction_RightClick _returnvalue_2)))
    (:then_2
      (Default|CallOnSelectedActionsChanged (Variables|Default|GetSelectedAction_LeftClick) (Variables|Default|GetSelectedAction_RightClick)))))